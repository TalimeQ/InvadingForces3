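; Player ship pawn that moves sideways by drag-planned steps and fires projectiles, working with the game mode's Sequencer.
; Dragging positions a lazily spawned helper actor, clamped on X to the current movement range.
; Releasing notifies the controller and sequence, then Tick moves and banks the ship toward that point using position and angle curves.
; Normal shots spawn at two ship sockets and register with the Sequencer; special shooting is an empty stub.
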(event `/Game/Blueprints/Core/BPi_ShootInterface.ShootSpecial`)

(event `/Game/Blueprints/Core/BPi_ShootInterface.ShootNormal`
  (for _array_element (`self.GetNormalShootingPoints`)
    (bind _returnvalue (`|SpawnActorFromClass` "/Game/Blueprints/Core/Projectiles/BP_BaseProjectile.BP_BaseProjectile_C" (`KismetMathLibrary.MakeTransform` _array_element (struct :`Yaw` -90.0)) "Undefined" "MultiplyWithRoot" null null))
    (bind _asbp_game_mode (cast `/Game/Blueprints/Core/BP_GameMode` (`GameplayStatics.GetGameMode`)))
    (`/Game/Blueprints/Sequencer/BP_SequencerBase.RegisterActor` (`/Game/Blueprints/Core/BP_GameMode.Sequencer` _asbp_game_mode) _returnvalue)))

(event `self.ReceiveBeginPlay`
  (bind _asbp_game_mode (cast `/Game/Blueprints/Core/BP_GameMode` (`GameplayStatics.GetGameMode`)))
  (`/Game/Blueprints/Core/BP_GameMode.GetSequencer` _asbp_game_mode))

(event `/Game/Blueprints/Core/BPI_MovementInterface.SetAvailableMovement`
  (params (MovementRange :type "Float (double-precision)") (Time :type "Float (double-precision)"))
  (set `self.CurrentMovementRange` (`KismetMathLibrary.FMax` MovementRange (`self.CurrentMovementRange`)))
  (set `self.MovementTime` Time)
  (set `self.RangePerSecond` (/ (`self.CurrentMovementRange`) (`self.MovementTime`))))

(event `self.ReceiveTick`
  (params (DeltaSeconds :type "Float (single-precision)"))
  (if (not (> (`self.CurrentMovementTime`) (`self.MovementTime`)))
    (bind _output_get (set `self.CurrentMovementTime` (+ DeltaSeconds (`self.CurrentMovementTime`))))
    (bind _returnvalue (/ _output_get (`self.MovementTime`)))
    (`self.K2_SetActorLocation` (`KismetMathLibrary.VLerp` (`self.StartPosition`) (`self.DragPosition`) (`CurveFloat.GetFloatValue` (`self.PositionCurve`) _returnvalue)))
    (`self.K2_SetActorRotation` (`KismetMathLibrary.RLerp` (struct :`Yaw` -90.0) (`KismetMathLibrary.MakeRotator` (`self.AngleRotation`) 0.0 -90.0) (`CurveFloat.GetFloatValue` (`self.AngleCurve`) _returnvalue)))))

(fn `FinishDrag`
  (message `/Game/Blueprints/Core/BPI_DragInterface.FinishDrag` (`GameplayStatics.GetPlayerController` 0))
  (`self.SetActorHiddenInGame` (`self.GetDragHelper`) true)
  (`self.OnSequenceFinished`)
  (set `self.CurrentMovementTime` 0.0)
  (set `self.StartPosition` (`self.K2_GetActorLocation`))
  (if (> (.x (`self.K2_GetActorLocation`)) (.x (`self.DragPosition`)))
    (set `self.AngleRotation` -25.0)
    (else
      (set `self.AngleRotation` 25.0))))

(fn `GetDragHelper`
  (returns (DragHelper :type "/Game/Blueprints/BP_DragHelper Object Reference"))
  (`/Engine/EditorBlueprintResources/StandardMacros.IsValid` (`self.DragHelper`)
    (:`Is Valid`
      (return (`self.DragHelper`)))
    (:`Is Not Valid`
      (bind _returnvalue (`|SpawnActorFromClass` "/Game/Blueprints/BP_DragHelper.BP_DragHelper_C" (`KismetMathLibrary.MakeTransform` (0.0 0.0 0.0)) "Undefined" "MultiplyWithRoot" null null))
      (bind _output_get (set `self.DragHelper` _returnvalue))
      (return _output_get))))

(fn `GetNormalShootingPoints`
  (returns (ShootPoints :type "Array of Vector Structure"))
  (return (`|MakeArray` (`SceneComponent.GetSocketLocation` (`self.player_ship`) "NormalShoot1") (`SceneComponent.GetSocketLocation` (`self.player_ship`) "NormalShoot2"))))

(fn `GetSpecialShootingPoints`
  (returns (SpecialShootPoints :type "Array of Vector Structure"))
  (return (`|MakeArray` (`SceneComponent.GetSocketLocation` (`self.player_ship`) "NormalShoot1") (`SceneComponent.GetSocketLocation` (`self.player_ship`) "NormalShoot2"))))

(fn `ProcessDrag`
  (params (Drag :type "Vector Structure"))
  (bind _draghelper (`self.GetDragHelper`))
  (bind _x (.x (`self.K2_GetActorLocation`)))
  (bind _returnvalue (`KismetMathLibrary.MakeVector` (`KismetMathLibrary.FClamp` (.x Drag) (- _x (`self.CurrentMovementRange`)) (+ _x (`self.CurrentMovementRange`))) (.y (`self.K2_GetActorLocation`)) (.z (`self.K2_GetActorLocation`))))
  (`self.K2_SetActorLocation` _draghelper _returnvalue false false)
  (`self.K2_SetActorRotation` _draghelper (struct :`Yaw` -90.0) false)
  (set `self.DragPosition` _returnvalue))

(fn `StartDrag`
  (`self.SetActorHiddenInGame` (`self.GetDragHelper`) false))

(fn `UserConstructionScript`)