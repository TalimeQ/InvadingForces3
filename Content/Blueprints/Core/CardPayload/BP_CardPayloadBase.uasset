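; BP_CardPayloadBase is a base Blueprint for timed card payloads, with an empty ExecutePayload function as the effect hook.
; TickPayload adds the passed time step to CurrentTime and calls ExecutePayload once the total reaches ExecutionStart.
; Multi-execute payloads then reset the timer to repeat, while others clear ShouldExecute, which TickPayload itself does not check.
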(fn `ExecutePayload`)

(fn `TickPayload`
  (params (TickPayload :type "Float (double-precision)"))
  (bind _returnvalue (+ (`self.CurrentTime`) TickPayload))
  (if (>= _returnvalue (`self.ExecutionStart`))
    (`self.ExecutePayload`)
    (if (`self.bIsMultiExecute`)
      (set `self.CurrentTime` 0.0)
      (else
        (set `self.ShouldExecute` false)))
    (else
      (set `self.CurrentTime` _returnvalue))))