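; Game mode that switches the first player's view to a level CameraActor, owns the sequencer actor and tracks score.
; BeginPlay and GetSequencer both spawn a BP_SequencerBase when none is valid; BeginPlay also resets Score, then calls UpdateScore, so it starts at one.
; UpdateScore increments Score and, like UpdatePlayerHp, pushes the value to the HUD through BP_PlayerController's HudRef.
; PlaySequence is an empty stub.
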(event `self.ReceiveBeginPlay`
  (bind _returnvalue (`GameplayStatics.GetActorOfClass` "/Script/Engine.CameraActor"))
  (`PlayerController.SetViewTargetWithBlend` (`GameplayStatics.GetPlayerController` 0) _returnvalue 0.0 "VTBlend_Linear" 0.0 false)
  (`/Engine/EditorBlueprintResources/StandardMacros.IsValid` (`self.Sequencer`)
    (:`Is Not Valid`
      (bind _returnvalue_2 (`|SpawnActorFromClass` "/Game/Blueprints/Sequencer/BP_SequencerBase.BP_SequencerBase_C" (`KismetMathLibrary.MakeTransform` (0.0 0.0 0.0)) "Undefined" "MultiplyWithRoot" null null))
      (set `self.Sequencer` _returnvalue_2)
      (set `self.Score` 0)
      (`self.UpdateScore`))))

(fn `GetSequencer`
  (returns (Sequencer :type "/Game/Blueprints/Sequencer/BP_SequencerBase Object Reference"))
  (`/Engine/EditorBlueprintResources/StandardMacros.IsValid` (`self.Sequencer`)
    (:`Is Valid`
      (return (`self.Sequencer`)))
    (:`Is Not Valid`
      (bind _returnvalue (`|SpawnActorFromClass` "/Game/Blueprints/Sequencer/BP_SequencerBase.BP_SequencerBase_C" (`KismetMathLibrary.MakeTransform` (0.0 0.0 0.0)) "Undefined" "MultiplyWithRoot" null null))
      (bind _output_get (set `self.Sequencer` _returnvalue))
      (return _output_get))))

(fn `Play Sequence`)

(fn `UpdatePlayerHp`
  (params (NewHp :type Integer))
  (bind _asbp_player_controller (cast `/Game/Blueprints/BP_PlayerController` (`GameplayStatics.GetPlayerController` 0)))
  (`/Game/Ui/CardUi/W_CardHUD.UpdateHP` (`/Game/Blueprints/BP_PlayerController.HudRef` _asbp_player_controller) (`local.NewHp`)))

(fn `UpdateScore`
  (`/Engine/EditorBlueprintResources/StandardMacros.IncrementInt` (`self.Score`)
    (:`  `
      (bind _asbp_player_controller (cast `/Game/Blueprints/BP_PlayerController` (`GameplayStatics.GetPlayerController` 0)))
      (`/Game/Ui/CardUi/W_CardHUD.UpdateScore` (`/Game/Blueprints/BP_PlayerController.HudRef` _asbp_player_controller) (`self.Score`)))))

(fn `UserConstructionScript`)