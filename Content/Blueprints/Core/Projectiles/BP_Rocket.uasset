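; BP_Rocket is a projectile that deals area damage when its Box overlaps an actor whose class is in PotentialTargets.
; A looping or long-running rocket sound is attached to the Cube on BeginPlay and kept for later stopping.
; On impact, a sphere overlap sends ProcessHitMessage to nearby world static and dynamic actors, skipping BP_PlayerPawn.
; It then stops the flight sound, plays an explosion at its location and calls DestroyObject.
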(event `self.ReceiveBeginPlay`
  (`parent.ReceiveBeginPlay`)
  (bind _returnvalue (`GameplayStatics.SpawnSoundAttached` "/Game/Sounds/698696__ienba__comet-asteroid-or-rocket.698696__ienba__comet-asteroid-or-rocket" (`self.Cube`) "None" (0.0 0.0 0.0) (struct) "KeepRelativeOffset" false 1.0 1.0 0.0 null null false))
  (set `self.Sound` _returnvalue))

(event `self.Box.OnComponentBeginOverlap`
  (params (OverlappedComponent :type "PrimitiveComponent Object Reference") (OtherActor :type "Actor Object Reference") (OtherComp :type "PrimitiveComponent Object Reference") (OtherBodyIndex :type Integer) (bFromSweep :type Boolean) (SweepResult :type "HitResult Structure (by ref)"))
  (if (`KismetArrayLibrary.Array_Contains` (`self.PotentialTargets`) (`GameplayStatics.GetObjectClass` OtherActor))
    (bind _outactors (`KismetSystemLibrary.SphereOverlapActors` (`self.K2_GetActorLocation`) 500.0 (`|MakeArray` "ObjectTypeQuery1" "ObjectTypeQuery2" :!type "EObjectTypeQuery Enum")))
    (for _array_element _outactors
      (cast `/Game/Blueprints/Core/BP_PlayerPawn` _array_element
        (:`CastFailed`
          (message `/Game/Blueprints/Core/BPI_HitInterface.ProcessHit` _array_element 5 "BP_Rocket_C" self false))))
    (`AudioComponent.Stop` (`self.Sound`))
    (`GameplayStatics.PlaySoundAtLocation` "/Game/Sounds/587174__derplayer__explosion_wide_edit.587174__derplayer__explosion_wide_edit" (`self.K2_GetActorLocation`) (struct) 1.0 1.0 0.0 null null null null)
    (`self.DestroyObject`)))

(fn `UserConstructionScript`
  (`parent.UserConstructionScript`))