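; Base sequencer that plays a card's payload mods over a timed sequence lasting the longest execution cost or the passed cost adjustment, whichever is greater.
; PlayCard targets mods at the player pawn; movement payloads hold execution, show movement range and begin a drag until StartSequence runs.
; Tick advances the mods and applies curve-driven CustomTimeDilation to registered actors, then clears the mods when time runs out.
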(event `self.ReceiveTick`
  (params (DeltaSeconds :type "Float (single-precision)"))
  (if (`self.ShouldExecute`)
    (if (>= (`self.CurrentTime`) (`self.SequenceTime`))
      (`self.FinishSequence`)
      (else
        (set `self.CurrentTime` (+ (`self.CurrentTime`) DeltaSeconds))
        (`self.Tick Mods` DeltaSeconds)
        (`self.TickTimescale`)))))

(fn `BindToPlayerPawn`
  (params (PlayerPawn :type "/Game/Blueprints/Core/BP_PlayerPawn Object Reference"))
  (add `/Game/Blueprints/Core/BP_PlayerPawn.OnSequenceFinished` PlayerPawn (`|CreateDelegate` :!event `Start Sequence`)))

(fn `FinishSequence`
  (set `self.ShouldExecute` false)
  (`KismetArrayLibrary.Array_Clear` (`self.Card Mods`))
  (set `self.IsPlayingSequence` false))

(fn `PlayCard`
  (params (CardMods :type "Array of /Game/Blueprints/Core/CardPayload/BP_CardPayloadBase Object Reference") (CardCostAdjustment :type "Float (double-precision)"))
  (locals (MaxTime :type "Float (double-precision)") (LocalShouldExecute :type Boolean))
  (set `self.IsPlayingSequence` true)
  (set `local.LocalShouldExecute` true)
  (for _array_element CardMods
    (bind _asbp_card_payload_move (cast `/Game/Blueprints/Core/CardPayload/BP_CardPayloadMove` _array_element))
    (set `local.LocalShouldExecute` false)
    (message `/Game/Blueprints/Core/BPI_MovementInterface.SetAvailableMovement` (`GameplayStatics.GetPlayerPawn` 0) (`/Game/Blueprints/Core/CardPayload/BP_CardPayloadMove.MovementRange` _asbp_card_payload_move) (`KismetMathLibrary.FMax` (`/Game/Blueprints/Core/CardPayload/BP_CardPayloadBase.ExecutionCost` _asbp_card_payload_move) (`local.CardCostAdjustment`)))
    (message `/Game/Blueprints/Core/BPI_DragInterface.StartDrag` (`GameplayStatics.GetPlayerController` 0)))
  (bind _output_get (set `self.Card Mods` CardMods))
  (set `local.MaxTime` CardCostAdjustment)
  (for _array_element_2 _output_get
    (set `local.MaxTime` (`KismetMathLibrary.FMax` (`/Game/Blueprints/Core/CardPayload/BP_CardPayloadBase.ExecutionCost` _array_element_2) (`local.MaxTime`)))
    (set `/Game/Blueprints/Core/CardPayload/BP_CardPayloadBase.ExecutingActor` (`Controller.K2_GetPawn` (`GameplayStatics.GetPlayerController` 0)) _array_element_2)
    (`/Game/Blueprints/Core/CardPayload/BP_CardPayloadBase.ResetExecute` _array_element_2))
  (set `self.CurrentTime` 0.0)
  (set `self.SequenceTime` (`local.MaxTime`))
  (set `self.ShouldExecute` (`local.LocalShouldExecute`)))

(fn `RegisterActor`
  (params (ActorToRegister :type "Actor Object Reference"))
  (`KismetArrayLibrary.Array_Add` (`self.RegisteredActors`) ActorToRegister))

(fn `Start Sequence`
  (set `self.ShouldExecute` true)
  (set `self.CurrentTime` 0.0))

(fn `Tick Mods`
  (params (DeltaTime :type "Float (double-precision)"))
  (for _array_element (`self.Card Mods`)
    (`/Game/Blueprints/Core/CardPayload/BP_CardPayloadBase.TickPayload` _array_element DeltaTime)))

(fn `TickTimescale`
  (locals (TimeDilation :type "Float (single-precision)" :default 0.0))
  (set `local.TimeDilation` (`CurveFloat.GetFloatValue` (`self.Curve`) (/ (`self.CurrentTime`) (`self.SequenceTime`))))
  (for _array_element (`self.RegisteredActors`)
    (set `Actor.CustomTimeDilation` (`local.TimeDilation`) _array_element)))

(fn `UnregisterActor`
  (params (ActorToRegister :type "Actor Object Reference"))
  (`KismetArrayLibrary.Array_RemoveItem` (`self.RegisteredActors`) ActorToRegister))

(fn `UserConstructionScript`)