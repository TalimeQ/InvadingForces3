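; BP_Meteor2 is an enemy meteor that flies along world Y at random speed, spinning with randomized scale.
; It registers with the game mode's sequencer and starts frozen at zero time dilation; DestroyObject unregisters and destroys it.
; Its mesh sends hit damage to overlapping actors.
; Player projectile hits reduce its health, but reaching zero triggers nothing.
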(event `self.ReceiveBeginPlay`
  (bind _returnvalue (`KismetMathLibrary.RandomFloatInRange` 0.2 0.5))
  (bind _asbp_game_mode (cast `/Game/Blueprints/Core/BP_GameMode` (`GameplayStatics.GetGameMode`)))
  (bind _sequencer (`/Game/Blueprints/Core/BP_GameMode.GetSequencer` _asbp_game_mode))
  (`/Game/Blueprints/Sequencer/BP_SequencerBase.RegisterActor` _sequencer self)
  (set `self.CustomTimeDilation` 0.0)
  (set `self.Speed` (`KismetMathLibrary.RandomFloatInRange` 600.0 1200.0))
  (set `self.RotationSpeed` (`KismetMathLibrary.RandomFloatInRange` 90.0 720.0))
  (`SceneComponent.K2_SetRelativeRotation` (`self.StaticMesh`) (`KismetMathLibrary.MakeRotator` (`KismetMathLibrary.RandomFloat`) (`KismetMathLibrary.RandomFloat`) (`KismetMathLibrary.RandomFloat`)) false false)
  (`SceneComponent.SetRelativeScale3D` (`self.StaticMesh`) (`KismetMathLibrary.MakeVector` _returnvalue _returnvalue _returnvalue)))

(event `self.ReceiveTick`
  (params (DeltaSeconds :type "Float (single-precision)"))
  (`SceneComponent.K2_AddWorldOffset` (`self.DefaultSceneRoot`) (`KismetMathLibrary.MakeVector` 0.0 (* DeltaSeconds (`self.Speed`))) false false)
  (`SceneComponent.K2_AddLocalRotation` (`self.StaticMesh`) (`KismetMathLibrary.MakeRotator` (* DeltaSeconds (`self.RotationSpeed`))) false false))

(event `self.DestroyObject`
  (bind _asbp_game_mode (cast `/Game/Blueprints/Core/BP_GameMode` (`GameplayStatics.GetGameMode`)))
  (bind _sequencer (`/Game/Blueprints/Core/BP_GameMode.GetSequencer` _asbp_game_mode))
  (`/Game/Blueprints/Sequencer/BP_SequencerBase.UnregisterActor` _sequencer self)
  (`self.K2_DestroyActor`))

(event `/Game/Blueprints/Core/BPI_HitInterface.ProcessHit`
  (params (Damage :type Integer) (HittingClass :type "Actor Class Reference") (HittingActor :type "Actor Object Reference"))
  (if (== HittingClass "/Game/Blueprints/Core/Projectiles/BP_ProjectilePlayer.BP_ProjectilePlayer_C")
    (bind _output_get (set `self.Health` (- (`self.Health`) Damage)))
    (if (<= _output_get 0)
      _)))

(event `self.StaticMesh.OnComponentBeginOverlap`
  (params (OverlappedComponent :type "PrimitiveComponent Object Reference") (OtherActor :type "Actor Object Reference") (OtherComp :type "PrimitiveComponent Object Reference") (OtherBodyIndex :type Integer) (bFromSweep :type Boolean) (SweepResult :type "HitResult Structure (by ref)"))
  (message `/Game/Blueprints/Core/BPI_HitInterface.ProcessHit` OtherActor 3 (`GameplayStatics.GetObjectClass` self) self))

(fn `UserConstructionScript`)