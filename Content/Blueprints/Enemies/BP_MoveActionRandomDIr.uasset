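; BP_MoveActionRandomDIr is an enemy move action that slides a pawn along X in a random direction while it fires at intervals.
; PrepareAction stores the start location and picks a signed, clamped X offset as the target.
; TickAction eases location and rotation with curves, though AngleRot is zeroed so pitch stays level.
; It calls ShootNormalMessage on each shoot interval and finishes once TimeInterval elapses.
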(fn `PrepareAction`
  (params (PawnRef :type "/Game/Blueprints/Enemies/BP_EnemyPawn Object Reference"))
  (locals (LocalDir :type "Float (double-precision)"))
  (`parent.PrepareAction` PawnRef)
  (bind _output_get (set `self.StartLocation` (`Actor.K2_GetActorLocation` (`self.PawnRef`))))
  (bind _output_get_2 (set `local.LocalDir` (* (`KismetMathLibrary.SelectInt` 1 -1 (`KismetMathLibrary.RandomBool`)) (`self.MovementValue`))))
  (set `self.DesiredLocation` (`KismetMathLibrary.MakeVector` (+ (.x _output_get) (`KismetMathLibrary.FClamp` _output_get_2 -270.0 1050.0)) (.y _output_get) (.z _output_get)))
  (set `self.AngleRot` 0.0))

(fn `TickAction`
  (params (DeltaTime :type "Float (double-precision)"))
  (set `self.ShootTime` (+ (`self.ShootTime`) DeltaTime))
  (bind _output_get (set `self.CurrentTime` (+ (`self.CurrentTime`) DeltaTime)))
  (if (> _output_get (`self.TimeInterval`))
    (`self.FinishExecute`)
    (else
      (if (> (`self.ShootTime`) (`self.ShootInterval`))
        (set `self.ShootTime` 0.0)
        (message `/Game/Blueprints/Core/BPi_ShootInterface.ShootNormal` (`self.PawnRef`)))
      (`Actor.K2_SetActorLocation` (`self.PawnRef`) (`KismetMathLibrary.VLerp` (`self.StartLocation`) (`self.DesiredLocation`) (`CurveFloat.GetFloatValue` (`self.MoveCurve`) (/ (`self.CurrentTime`) (`self.TimeInterval`)))) false false)
      (`Actor.K2_SetActorRotation` (`self.PawnRef`) (`KismetMathLibrary.RLerp` (struct :`Yaw` -180.0) (`KismetMathLibrary.MakeRotator` 0.0 (`self.AngleRot`) -180.0) (`CurveFloat.GetFloatValue` (`self.AngleCurve`) (/ (`self.CurrentTime`) (`self.TimeInterval`)))) false))))