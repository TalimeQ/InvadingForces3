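; Enemy and meteor spawner that places actors at a random X along the Y position of its Box component.
; It registers with the game mode's sequencer and starts frozen at zero time dilation.
; A Tick timer spawns one of three random meteor classes at randomized intervals.
; RespawnEnemy updates the score, resets and relocates the given enemy, and randomly spawns an additional BP_EnemyPawn.
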(event `self.ReceiveBeginPlay`
  (bind _asbp_game_mode (cast `/Game/Blueprints/Core/BP_GameMode` (`GameplayStatics.GetGameMode`)))
  (bind _sequencer (`/Game/Blueprints/Core/BP_GameMode.GetSequencer` _asbp_game_mode))
  (`/Game/Blueprints/Sequencer/BP_SequencerBase.RegisterActor` _sequencer self)
  (set `self.CustomTimeDilation` 0.0)
  (set `self.TimeTillEvent` (`KismetMathLibrary.RandomFloatInRange` (`self.Min`) (`self.Max`))))

(event `self.ReceiveTick`
  (params (DeltaSeconds :type "Float (single-precision)"))
  (set `self.CurrentTime` (+ (`self.CurrentTime`) DeltaSeconds))
  (if (> (`self.CurrentTime`) (`self.TimeTillEvent`))
    (`self.SpawnRandomEvent`)))

(fn `RespawnEnemy`
  (params (Actor :type "/Game/Blueprints/Enemies/BP_EnemyPawn Object Reference"))
  (bind _asbp_game_mode (cast `/Game/Blueprints/Core/BP_GameMode` (`GameplayStatics.GetGameMode`))
    (:`then`
      (`/Game/Blueprints/Core/BP_GameMode.UpdateScore` _asbp_game_mode))
    (:`CastFailed`
      _))
  (set `/Game/Blueprints/Enemies/BP_EnemyPawn.Health` 2 Actor)
  (`self.K2_SetActorLocation` Actor (`KismetMathLibrary.MakeVector` (`KismetMathLibrary.RandomFloatInRange` 0.0 1050.0) (.y (`SceneComponent.K2_GetComponentLocation` (`self.Box`))) 120.0) false false)
  (if (`KismetMathLibrary.RandomBool`)
    (`|SpawnActorFromClass` "/Game/Blueprints/Enemies/BP_EnemyPawn.BP_EnemyPawn_C" (`KismetMathLibrary.MakeTransform` (`KismetMathLibrary.MakeVector` (`KismetMathLibrary.RandomFloatInRange` 0.0 1050.0) (.y (`SceneComponent.K2_GetComponentLocation` (`self.Box`))) 120.0)) "Undefined" "MultiplyWithRoot" null null)))

(fn `SpawnRandomEvent`
  (set `self.TimeTillEvent` (`KismetMathLibrary.RandomFloatInRange` 5.0 12.0))
  (set `self.CurrentTime` 0.0)
  (`|SpawnActorFromClass` (`KismetArrayLibrary.Array_Random` (`|MakeArray` "/Game/Blueprints/Enemies/BP_Meteor.BP_Meteor_C" "/Game/Blueprints/Enemies/BP_Meteor2.BP_Meteor2_C" "/Game/Blueprints/Enemies/BP_Meteor3.BP_Meteor3_C" :!type "Actor Class Reference")) (`KismetMathLibrary.MakeTransform` (`KismetMathLibrary.MakeVector` (`KismetMathLibrary.RandomFloatInRange` 0.0 1050.0) (.y (`SceneComponent.K2_GetComponentLocation` (`self.Box`))) 120.0)) "Undefined" "MultiplyWithRoot"))

(fn `UserConstructionScript`
  (`BoxComponent.SetBoxExtent` (`self.Box`) (`self.In Box Extent`) true))