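; Enemy pawn that runs randomly chosen action objects, fires projectiles and takes damage from player projectiles and rockets.
; It starts itself and its projectiles at zero time dilation and registers them with the game mode's sequencer.
; Actions built from PossibleActions tick on the pawn, with later picks biased toward the last two entries.
; At zero health it explodes, is handed to BP_ActorSpawner for respawn and picks a new action.
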(event `self.ReceiveBeginPlay`
  (set `self.CustomTimeDilation` 0.0)
  (`self.K2_SetActorRotation` (struct :`Yaw` -180.0))
  (bind _asbp_game_mode (cast `/Game/Blueprints/Core/BP_GameMode` (`GameplayStatics.GetGameMode`)))
  (bind _sequencer (`/Game/Blueprints/Core/BP_GameMode.GetSequencer` _asbp_game_mode))
  (`/Game/Blueprints/Sequencer/BP_SequencerBase.RegisterActor` _sequencer self)
  (for _array_element (`self.PossibleActions`)
    (bind _returnvalue (`|GenericCreateObject` _array_element))
    (`KismetArrayLibrary.Array_Add` (`self.GeneratedActions`) _returnvalue))
  (bind _output_get (set `self.CurrentAction` (`KismetArrayLibrary.Array_Random` (`self.GeneratedActions`))))
  (`/Game/Blueprints/Enemies/EnemyActionBase.PrepareAction` _output_get self)
  (bind _returnvalue_2 (`GameplayStatics.GetActorOfClass` "/Game/Blueprints/Enemies/BP_ActorSpawner.BP_ActorSpawner_C"))
  (set `self.Spawner` _returnvalue_2))

(event `self.ReceiveTick`
  (params (DeltaSeconds :type "Float (single-precision)"))
  (`/Engine/EditorBlueprintResources/StandardMacros.IsValid` (`self.CurrentAction`)
    (:`Is Valid`
      (`/Game/Blueprints/Enemies/EnemyActionBase.TickAction` (`self.CurrentAction`) DeltaSeconds))))

(event `/Game/Blueprints/Core/BPi_ShootInterface.ShootSpecial`)

(event `/Game/Blueprints/Core/BPi_ShootInterface.ShootNormal`
  (bind _returnvalue (`|SpawnActorFromClass` "/Game/Blueprints/Enemies/BP_ProjectileEnemy.BP_ProjectileEnemy_C" (`KismetMathLibrary.MakeTransform` (`KismetArrayLibrary.Array_Random` (`self.GetRandomShootPos`)) (struct :`Yaw` 90.0)) "Undefined" "MultiplyWithRoot" null null))
  (set `Actor.CustomTimeDilation` 0.0 _returnvalue)
  (bind _asbp_game_mode (cast `/Game/Blueprints/Core/BP_GameMode` (`GameplayStatics.GetGameMode`)))
  (bind _sequencer (`/Game/Blueprints/Core/BP_GameMode.GetSequencer` _asbp_game_mode))
  (`/Game/Blueprints/Sequencer/BP_SequencerBase.RegisterActor` _sequencer _returnvalue)
  (`GameplayStatics.PlaySoundAtLocation` "/Game/Sounds/234082__211redman112__lasgun-impact.234082__211redman112__lasgun-impact" (`self.K2_GetActorLocation`) (struct) 1.0 1.0 0.0 null null null null))

(event `/Game/Blueprints/Objects/BPI_ObjectDestroyer.DestroyObject`
  (`/Game/Blueprints/Enemies/BP_ActorSpawner.RespawnEnemy` (`self.Spawner`) self)
  (`self.ClearBinds` (`self.CurrentAction`))
  (`self.Process Next Action`))

(event `/Game/Blueprints/Core/BPI_HitInterface.ProcessHit`
  (params (Damage :type Integer) (HittingClass :type "Actor Class Reference") (HittingActor :type "Actor Object Reference") (ShouldDestroy :type Boolean))
  (bind _returnvalue (`self.K2_GetActorLocation`))
  (if (or (== HittingClass "/Game/Blueprints/Core/Projectiles/BP_ProjectilePlayer.BP_ProjectilePlayer_C") (== HittingClass "/Game/Blueprints/Core/Projectiles/BP_Rocket.BP_Rocket_C"))
    (if ShouldDestroy
      (message `/Game/Blueprints/Objects/BPI_ObjectDestroyer.DestroyObject` HittingActor))
    (bind _output_get (set `self.Health` (- (`self.Health`) Damage)))
    (if (<= _output_get 0)
      (`GameplayStatics.SpawnSoundAtLocation` "/Game/Sounds/244394__werra__bangexplosion-metallic.244394__werra__bangexplosion-metallic" _returnvalue (struct) 1.0 1.0 0.0 null null)
      (`GameplayStatics.SpawnEmitterAtLocation` "/Game/Realistic_Starter_VFX_Pack_Vol2/Particles/Explosion/P_Explosion_Big_B.P_Explosion_Big_B" _returnvalue)
      (`/Game/Blueprints/Objects/BPI_ObjectDestroyer.DestroyObject`))))

(fn `ClearBinds`
  (params (Action :type "/Game/Blueprints/Enemies/EnemyActionBase Object Reference"))
  (clear `/Game/Blueprints/Enemies/EnemyActionBase.ActionFinished` Action))

(fn `GetPossibleAction`)

(fn `GetRandomShootPos`
  (returns (ShootPositions :type "Array of Vector Structure"))
  (bind _staticmesh1 (`self.StaticMesh1`))
  (return (`|MakeArray` (`SceneComponent.GetSocketLocation` _staticmesh1 "None") (`SceneComponent.GetSocketLocation` _staticmesh1 "None"))))

(fn `Process Next Action`
  (bind _generatedactions (`self.GeneratedActions`))
  (if (`KismetMathLibrary.RandomBool`)
    (bind _output_get (set `self.CurrentAction` (`KismetArrayLibrary.Array_Random` (`self.GeneratedActions`))))
    (else
      (set `self.CurrentAction` (`|GetArrayItem` _generatedactions (- (`KismetArrayLibrary.Array_LastIndex` _generatedactions) (`KismetMathLibrary.SelectInt` 0 1 (`KismetMathLibrary.RandomBool`)))))))
  (`/Game/Blueprints/Enemies/EnemyActionBase.PrepareAction` _output_get self))

(fn `SetupBinds`
  (params (Action :type "/Game/Blueprints/Enemies/EnemyActionBase Object Reference"))
  (add `/Game/Blueprints/Enemies/EnemyActionBase.ActionFinished` Action (`|CreateDelegate` :!event `Process Next Action`)))

(fn `UserConstructionScript`)