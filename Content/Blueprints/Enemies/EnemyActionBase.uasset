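; Base enemy action that runs an overridable, empty ExecuteAction at a fixed time interval for a limited count.
; PrepareAction stores the pawn, has it set up binds to the action, and resets the timer and counter.
; TickAction accumulates delta time and fires each execution, running NumExecutions plus one in total before finishing.
; FinishExecute signals that the action finished, then clears the pawn's binds.
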(fn `ExecuteAction`)

(fn `FinishExecute`
  (`self.ActionFinished`)
  (`/Game/Blueprints/Enemies/BP_EnemyPawn.ClearBinds` (`self.PawnRef`) self))

(fn `PrepareAction`
  (params (PawnRef :type "/Game/Blueprints/Enemies/BP_EnemyPawn Object Reference"))
  (bind _output_get (set `self.PawnRef` PawnRef))
  (`/Game/Blueprints/Enemies/BP_EnemyPawn.SetupBinds` _output_get self)
  (set `self.CurrentTime` 0.0)
  (set `self.CurrentExecutionsNum` 0))

(fn `TickAction`
  (params (DeltaTime :type "Float (double-precision)"))
  (bind _output_get (set `self.CurrentTime` (+ (`self.CurrentTime`) DeltaTime)))
  (if (> _output_get (`self.TimeInterval`))
    (if (>= (`self.CurrentExecutionsNum`) (`self.NumExecutions`))
      (`self.ExecuteAction`)
      (`self.FinishExecute`)
      (else
        (`self.ExecuteAction`)
        (`/Engine/EditorBlueprintResources/StandardMacros.IncrementInt` (`self.CurrentExecutionsNum`)
          (:`  `
            (set `self.CurrentTime` 0.0)))))))