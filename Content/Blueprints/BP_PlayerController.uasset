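; Player controller that creates the card HUD, shows the mouse cursor and handles mouse dragging of player pawns.
; StartDrag and FinishDrag events toggle a flag that lets a left click hook a BP_PlayerPawn through a line trace from the cursor.
; Tick feeds the hooked pawn the cursor's hit location on WorldStatic objects until the button is released.
; Escape quits the game and R reloads MainLevel.
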(event EventBeginPlay
  (bind _returnvalue (UserInterface|CreateWidget "/Game/Ui/CardUi/W_CardHUD.W_CardHUD_C" self))
  (Variables|Default|SetHudRef _returnvalue)
  (UserInterface|Viewport|AddtoViewport _returnvalue 0)
  (Input|SetInputModeGameandUI self _returnvalue "DoNotLock" false false)
  (Variables|Default|SetbShowMouseCursor true))

(event EventTick
  (params (DeltaSeconds :type Float%20%28single-precision%29))
  (bind _hookedplayer (Variables|Default|GetHookedPlayer))
  (Utilities|IsValid _hookedplayer
    (:Is%20Valid
      (Default|ProcessDrag _hookedplayer (.Location (Collision|BreakHitResult (.HitResult (Class|PlayerController|GetHitResultUnderCursorforObjects (Utilities|Array|MakeArray "ObjectTypeQuery1") true))))))))

(event EventFinishDrag
  (Variables|Default|SetAwaitsDrag false))

(event EventStartDrag
  (Variables|Default|SetAwaitsDrag true))

(event Input|MouseEvents|DebugKeyLeftMouseButton
  (params (Key :type Key%20Structure :default "None") (ActionValue :type Input%20Action%20Value%20Structure))
  (bind (_worldlocation _worlddirection) (Game|Player|ConvertMouseLocationToWorldSpace))
  (bind _awaitsdrag (Variables|Default|GetAwaitsDrag))
  (:Pressed
    (if _awaitsdrag
      (bind (_outhit _returnvalue) (Collision|LineTraceForObjects _worldlocation (+ _worldlocation (* _worlddirection "10000.000000,10000.000000,10000.000000")) (Utilities|Array|MakeArray "ObjectTypeQuery2") false 0 "None" true "(R=1.000000,G=0.000000,B=0.000000,A=1.000000)" "(R=0.000000,G=1.000000,B=0.000000,A=1.000000)" 15.0))
      (if _returnvalue
        (bind _asbp_player_pawn (Utilities|Casting|CastToBP_PlayerPawn (.HitActor (Collision|BreakHitResult _outhit))))
        (bind _output_get (Variables|Default|SetHookedPlayer _asbp_player_pawn))
        (Default|StartDrag _output_get))))
  (:Released
    (if _awaitsdrag
      (Default|FinishDrag (Variables|Default|GetHookedPlayer))
      (Variables|Default|SetHookedPlayer 0))))

(event Input|KeyboardEvents|Escape
  (params (Key :type Key%20Structure :default "None"))
  (:Pressed
    (Game|QuitGame 0 "Quit" false)))

(event Input|KeyboardEvents|R
  (params (Key :type Key%20Structure :default "None"))
  (:Pressed
    (Game|OpenLevel(byName) "MainLevel")))

(fn ConstructionScript)